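; AC_Health is an actor component that tracks health and death state for its owner.
; Damage and healing apply only while alive, and reset restores full health only when dead.
; All changes route through one function that clamps health between zero and max, broadcasts OnHealthChanged, sets IsDead, and fires OnDead when health reaches zero.
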(event EventTakeDamage
  (params (Damage%20Amount :type Float%20%28double-precision%29))
  (if (not (Variables|Default|GetIsDead))
    (CallFunction|UpdateHealthandNotify (- (Variables|Default|GetCurrentHealth) Damage%20Amount))))

(event EventGainHealth
  (params (Health%20Gain%20Amount :type Float%20%28double-precision%29))
  (if (not (Variables|Default|GetIsDead))
    (CallFunction|UpdateHealthandNotify (+ (Variables|Default|GetCurrentHealth) Health%20Gain%20Amount))))

(event EventResetHealth
  (if (Variables|Default|GetIsDead)
    (CallFunction|UpdateHealthandNotify (Variables|Default|GetMaxHealth))))

(fn UpdateHealthandNotify
  (params (NewHealthValue :type Float%20%28double-precision%29))
  (Variables|Default|SetCurrentHealth (Math|Float|Clamp(Float) NewHealthValue 0.0 (Variables|Default|GetMaxHealth)))
  (Default|CallOnHealthChanged (Variables|Default|GetCurrentHealth) (Variables|Default|GetMaxHealth))
  (if (<= (Variables|Default|GetCurrentHealth) 0.0)
    (Variables|Default|SetIsDead true)
    (Default|CallOnDead)
    (else
      (Variables|Default|SetIsDead false))))