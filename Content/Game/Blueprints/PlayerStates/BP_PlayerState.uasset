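; BP_PlayerState is the player state that owns the player's health through the ACHealth component and persists it in BP_GameInstance.
; On BeginPlay it restores current and max health from the game instance, or resets and saves them on first initialization.
; Health changes are written back to the game instance, and death asks BP_ThirdPersonGameMode to start a respawn for the player controller.
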(event Custom|OnHealthChanged
  (params (CurrentHealth :type Float%20%28double-precision%29) (MaxHealth :type Float%20%28double-precision%29))
  (CallFunction|SaveHealth))

(event Custom|OnDead
  (bind _asbp_third_person_game_mode (Utilities|Casting|CastToBP_ThirdPersonGameMode (Game|GetGameMode)))
  (Default|StartRespawn _asbp_third_person_game_mode (Game|GetPlayerController)))

(event EventBeginPlay
  (bind _ac_health (Variables|Default|GetAC_Health))
  (EventDispatchers|BindEventtoOnDead (Variables|Default|GetAC_Health) (delegate Custom|OnDead))
  (EventDispatchers|BindEventtoOnHealthChanged (Variables|Default|GetAC_Health) (delegate Custom|OnHealthChanged))
  (bind _asbp_game_instance (Utilities|Casting|CastToBP_GameInstance (Game|GetGameInstance)))
  (bind _output_get (Variables|Default|SetBP%20Game%20Instance _asbp_game_instance))
  (if (Variables|/Game/Game/Blueprints/BP_GameInstance.BP_GameInstance_C|GetHealthInitialized _output_get)
    ;[0.15 0.15 0.15 0.5] Set max health to what is in GI
    (Variables|/Game/Game/Blueprints/Actors/AC_Health.AC_Health_C|SetMaxHealth _ac_health (Variables|/Game/Game/Blueprints/BP_GameInstance.BP_GameInstance_C|GetMaxHealth_GI (Variables|Default|GetBP%20Game%20Instance)))
    ;[0.15 0.15 0.15 0.5] Set Health to what is in GI
    (Default|UpdateHealthandNotify _ac_health (Variables|/Game/Game/Blueprints/BP_GameInstance.BP_GameInstance_C|GetCurrentHealth_GI (Variables|Default|GetBP%20Game%20Instance)))
    (else
      (Variables|/Game/Game/Blueprints/BP_GameInstance.BP_GameInstance_C|SetHealthInitialized (Variables|Default|GetBP%20Game%20Instance) true)
      (Default|ResetHealth (Variables|Default|GetAC_Health))
      (CallFunction|SaveHealth))))

(fn ConstructionScript)

(fn SaveHealth
  (bind _bp_game_instance (Variables|Default|GetBP%20Game%20Instance))
  (bind _ac_health (Variables|Default|GetAC_Health))
  (Variables|/Game/Game/Blueprints/BP_GameInstance.BP_GameInstance_C|SetCurrentHealth_GI _bp_game_instance (Variables|/Game/Game/Blueprints/Actors/AC_Health.AC_Health_C|GetCurrentHealth _ac_health))
  (Variables|/Game/Game/Blueprints/BP_GameInstance.BP_GameInstance_C|SetMaxHealth_GI _bp_game_instance (Variables|/Game/Game/Blueprints/Actors/AC_Health.AC_Health_C|GetMaxHealth _ac_health)))